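; BP_BaseTrrap is a trap that damages the player and sends them back to their last platform.
; It caches the BP_pLayer2D character on BeginPlay and reacts only when that player begins overlapping its Hitbox.
; On overlap it applies BaseDamage, then restores the player's transform from their stored LastPlatformPose.
; The construction script sizes the Hitbox from the InBoxExtent variable.
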(event OnComponentBeginOverlap(hitbox)
  (params (OverlappedComponent :type Primitive%20Component%20Object%20Reference) (OtherActor :type Actor%20Object%20Reference) (OtherComp :type Primitive%20Component%20Object%20Reference) (OtherBodyIndex :type Integer) (bFromSweep :type Boolean) (SweepResult :type Hit%20Result%20Structure%20%28by%20ref%29))
  (bind _player_ref (Variables|Default|GetPlayer%20ref))
  (bind _last_platform_pose (Variables|/Game/Blueprrints/BP_pLayer2D.BP_pLayer2D_C|GetLast%20Platform%20pose _player_ref))
  (if (== OtherActor (Variables|Default|GetPlayer%20ref))
    (Game|Damage|ApplyDamage (Variables|Default|GetPlayer%20ref) (Variables|Default|GetBase%20Damage) 0 0)
    (Transformation|SetActorTransform _player_ref (Math|Transform|MakeTransform (.location _last_platform_pose) (.rotation _last_platform_pose) (.scale _last_platform_pose)))))

(event EventBeginPlay
  (bind _asbp_p_layer_2d (Utilities|Casting|CastToBP_pLayer2D (Game|GetPlayerCharacter 0)))
  (Variables|Default|SetPlayer%20ref _asbp_p_layer_2d))

(fn ConstructionScript
  (Components|Box|SetBoxExtent (Variables|Default|Gethitbox) (Variables|Default|GetIn%20Box%20Extent) true))