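; BP_saveposition is a trigger volume that records a last platform position for the 2D player character, BP_pLayer2D.
; On BeginPlay it caches a reference to the player character.
; When that player overlaps the box, it writes the volume's own actor transform, rather than the player's, into the player's LastPlatformPose.
; The construction script sizes the box from the InBoxExtent variable.
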(event OnComponentBeginOverlap(Box)
  (params (OverlappedComponent :type Primitive%20Component%20Object%20Reference) (OtherActor :type Actor%20Object%20Reference) (OtherComp :type Primitive%20Component%20Object%20Reference) (OtherBodyIndex :type Integer) (bFromSweep :type Boolean) (SweepResult :type Hit%20Result%20Structure%20%28by%20ref%29))
  (if (== OtherActor (Variables|Default|Getplayerrref))
    (Variables|/Game/Blueprrints/BP_pLayer2D.BP_pLayer2D_C|SetLast%20Platform%20pose (Variables|Default|Getplayerrref) (Transformation|GetActorTransform))))

(event EventBeginPlay
  (bind _asbp_p_layer_2d (Utilities|Casting|CastToBP_pLayer2D (Game|GetPlayerCharacter 0)))
  (Variables|Default|Setplayerrref _asbp_p_layer_2d))

(fn ConstructionScript
  (Components|Box|SetBoxExtent (Variables|Default|GetBox) (Variables|Default|GetIn%20Box%20Extent) true))