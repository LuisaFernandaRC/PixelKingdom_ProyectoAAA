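; BP_EnemyBase is an enemy base Blueprint that handles health, damage intake and death.
; The construction script seeds current health and damage from their maximums, and BeginPlay caches the BP_pLayer2D player character.
; AnyDamage lowers health with a floor of zero; at zero it jumps the anim instance to the configured death node, disables capsule collision, detaches the controller and destroys the actor after a delay.
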(event EventBeginPlay
  (bind _asbp_p_layer_2d (Utilities|Casting|CastToBP_pLayer2D (Game|GetPlayerCharacter 0)))
  (Variables|Default|SetPlayer%20Ref _asbp_p_layer_2d))

(event Game|Damage|EventAnyDamage
  (params (Damage :type Float%20%28single-precision%29) (DamageType :type Damage%20Type%20Object%20Reference) (InstigatedBy :type Controller%20Object%20Reference) (DamageCauser :type Actor%20Object%20Reference))
  ;[1 1 1] Enemy dead
  (bind _output_get (Variables|Default|SetCurrent%20Health (Math|Float|Clamp(Float) (- (Variables|Default|GetCurrent%20Health) Damage) 0.0 (- (Variables|Default|GetCurrent%20Health) Damage))))
  (if (== _output_get 0.0)
    (Variables|Default|SetIsdead true)
    (if (Variables|Default|GetIsdead)
      (Class|PaperZDAnimInstance|JumptoNode (Class|PaperZDCharacter|GetAnimInstance) (Variables|Default|GetDead%20Anim%20Name) "None")
      (Collision|SetCollisionEnabled (Variables|Default|GetCapsuleComponent) "NoCollision")
      (Class|Pawn|DetachfromControllerPendingDestroy)
      (Utilities|FlowControl|Delay 5.0)
      (Actor|DestroyActor))))

(fn ConstructionScript
  (Variables|Default|SetCurrent%20Health (Variables|Default|GetMax%20Health))
  (Variables|Default|SetCurrent%20Damage (Variables|Default|GetMax%20Damage)))