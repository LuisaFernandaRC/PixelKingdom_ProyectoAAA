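; Projectile actor that damages enemies derived from BP_EnemyBase and destroys itself on impact.
; When HitBox overlaps an enemy, it applies BaseDamage, destroys the projectile and prints the damage result as debug output.
; Every Tick, a Visibility line trace from the actor to the Endtrace component, drawn for debugging, destroys the projectile on any hit without applying damage.
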(event OnComponentBeginOverlap(HitBox)
  (params (OverlappedComponent :type Primitive%20Component%20Object%20Reference) (OtherActor :type Actor%20Object%20Reference) (OtherComp :type Primitive%20Component%20Object%20Reference) (OtherBodyIndex :type Integer) (bFromSweep :type Boolean) (SweepResult :type Hit%20Result%20Structure%20%28by%20ref%29))
  (bind _asbp_enemy_base (Utilities|Casting|CastToBP_EnemyBase OtherActor))
  (bind _output_get (Variables|Default|SetAs%20BP%20Enemy%20Base _asbp_enemy_base))
  (bind _returnvalue (Game|Damage|ApplyDamage _output_get (Variables|Default|GetbaseDamage) 0 0))
  (Actor|DestroyActor)
  (Development|PrintString (Utilities|String|ToString(Float) _returnvalue)))

(event EventTick
  (params (DeltaSeconds :type Float%20%28single-precision%29))
  (bind _returnvalue (Collision|LineTraceByChannel (Transformation|GetActorLocation) (Transformation|GetWorldLocation (Variables|Default|GetEndtrace)) "TraceTypeQuery1" false 0 "ForOneFrame"))
  (if _returnvalue
    (Actor|DestroyActor)))

(fn ConstructionScript)